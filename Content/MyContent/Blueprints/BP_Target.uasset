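; BP_Target is a moving target actor that takes hits and destroys itself when its hit points run out.
; Tick offsets it along the normalized Direction by Speed each frame, without delta-time scaling or sweep.
; A looping timer started on BeginPlay negates Direction every MovementDuration, producing back-and-forth motion.
; Each call to the Hit event removes one hit point.
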(event `self.ReceiveBeginPlay`
  ;[0.04249 0.06131 0.15 0.5] Flip Direction
  (`KismetSystemLibrary.K2_SetTimerDelegate` (delegate `Event FlipDirection`) (`self.MovementDuration`) true))

(event `self.ReceiveHit`
  (params (MyComp :type "PrimitiveComponent Object Reference") (Other :type "Actor Object Reference") (OtherComp :type "PrimitiveComponent Object Reference") (bSelfMoved :type Boolean) (HitLocation :type "Vector Structure") (HitNormal :type "Vector Structure") (NormalImpulse :type "Vector Structure") (Hit :type "HitResult Structure (by ref)"))
  ;[0.15 0.07129 0.09176 0.5] Target Hit
  (set `self.HitPoint` (- (`self.HitPoint`) 1))
  (if (<= (`self.HitPoint`) 0)
    (`self.K2_DestroyActor`)))

(event `Event FlipDirection`
  ;[0.04249 0.06131 0.15 0.5] Flip Direction
  (set `self.Direction` (* (`self.Direction`) -1.0)))

(event `self.ReceiveTick`
  (params (DeltaSeconds :type "Float (single-precision)"))
  ;[0.06105 0.15 0.0739 0.5] Target Movement
  (`self.K2_AddActorWorldOffset` (* (`KismetMathLibrary.Normal` (`self.Direction`)) (`self.Speed`))))

(fn `UserConstructionScript`)